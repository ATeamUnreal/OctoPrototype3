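; Player controller for the TPS start screen, which shows the start widget with a mouse cursor and game-and-UI input.
; On BeginPlay it creates a settings save object and asks BP_GI for the local IP, printing it in debug mode.
; OpenLobby hands off to BP_GI to open a listen lobby.
; SaveIP and LoadIP persist the last IP address through the BP_SaveSettings save slot.
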(event `self.ReceiveBeginPlay`
  (bind _returnvalue (`GameplayStatics.CreateSaveGameObject` "/Game/Blueprints/System/TPSStart/BP_SaveSettings.BP_SaveSettings_C"))
  (set `self.SaveSettingsInstance` _returnvalue)
  (bind _returnvalue_2 (`|CreateWidget` "/Game/Blueprints/System/TPSStart/TPSStartWidget.TPSStartWidget_C"))
  (set `self.TPSStartWidget` _returnvalue_2)
  (`UserWidget.AddToViewport` (`self.TPSStartWidget`) 0)
  (set `self.bShowMouseCursor` true)
  (`WidgetBlueprintLibrary.SetInputMode_GameAndUIEx` self null)
  (bind _asbp_gi (cast `/Game/Blueprints/Public/BP_GI` (`GameplayStatics.GetGameInstance`)))
  (bind _returnvalue_3 (`MyGameInstance.GetMyIpAddress` _asbp_gi))
  (if (`/Game/Blueprints/Public/BP_GI.IsDebugMode` _asbp_gi)
    (`KismetSystemLibrary.PrintString` _returnvalue_3 true true (struct :`G` 0.66 :`B` 1.0 :`A` 1.0) 10.0)))

(event `OpenLobby`
  (bind _asbp_gi (cast `/Game/Blueprints/Public/BP_GI` (`GameplayStatics.GetGameInstance`)))
  (`/Game/Blueprints/Public/BP_GI.OpenLobby_Listen` _asbp_gi))

(fn `LoadIP`
  (returns (LastIPAddress :type String))
  (bind _returnvalue (`GameplayStatics.LoadGameFromSlot` (`/Game/Blueprints/System/TPSStart/BP_SaveSettings.SaveSlotName` (stale _output_get))))
  (bind _asbp_save_settings (cast `/Game/Blueprints/System/TPSStart/BP_SaveSettings` _returnvalue))
  (`/Engine/EditorBlueprintResources/StandardMacros.IsValid` _asbp_save_settings
    (:`Is Valid`
      (bind _output_get (set `self.SaveSettingsInstance` _asbp_save_settings))
      (return (`/Game/Blueprints/System/TPSStart/BP_SaveSettings.LastIPAddress` _output_get)))))

(fn `SaveIP`
  (params (NewIP :type String))
  (bind _savesettingsinstance (`self.SaveSettingsInstance`))
  (set `/Game/Blueprints/System/TPSStart/BP_SaveSettings.LastIPAddress` NewIP _savesettingsinstance)
  (`GameplayStatics.SaveGameToSlot` _savesettingsinstance (`/Game/Blueprints/System/TPSStart/BP_SaveSettings.SaveSlotName` _savesettingsinstance)))

(fn `UserConstructionScript`)